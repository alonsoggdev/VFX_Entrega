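; BP_InteractiveElement is an actor that drives its mesh material's opacity parameter by how close the third-person character is.
; Actor overlap events toggle InRange, with no filter on the overlapping actor.
; While in range, Tick divides character-to-mesh distance by the SphereTrigger radius, clamps it to 0–1 and writes it to OpacityControl.
; Tick also looks up the character and calls CreateDynamicMaterialInstance each frame, without caching either.
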(event `self.ReceiveTick`
  (params (DeltaSeconds :type "Float (single-precision)"))
  (if (`self.InRange`)
    (bind _returnvalue (`GameplayStatics.GetActorOfClass` "/Game/ThirdPerson/Blueprints/BP_ThirdPersonCharacter.BP_ThirdPersonCharacter_C"))
    (set `self.Distance` (`KismetMathLibrary.FClamp` (/ (`KismetMathLibrary.Vector_Distance` (`SceneComponent.K2_GetComponentLocation` (`self.StaticMesh`)) (`self.K2_GetActorLocation` _returnvalue)) (`SphereComponent.SphereRadius` (`self.SphereTrigger`)))))
    (bind _returnvalue_2 (`PrimitiveComponent.CreateDynamicMaterialInstance` (`self.StaticMesh`) 0 null "None"))
    (`MaterialInstanceDynamic.SetScalarParameterValue` _returnvalue_2 "OpacityControl" (`self.Distance`))))

(event `self.ReceiveActorBeginOverlap`
  (params (OtherActor :type "Actor Object Reference"))
  (set `self.InRange` true))

(event `self.ReceiveActorEndOverlap`
  (params (OtherActor :type "Actor Object Reference"))
  (set `self.InRange` false))

(fn `UserConstructionScript`)